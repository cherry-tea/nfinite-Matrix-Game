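; BP_Shoot is a projectile that destroys enemies and awards score to the player.
; Tick raises its speed by a fixed step each frame and moves it along world X with teleport, printing the speed.
; When its sphere overlaps a BP_Enemy, it destroys the enemy and itself, then adds points to BP_Player's Score once via DoOnce and prints the total.
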(event `self.ReceiveTick`
  (params (DeltaSeconds :type "Float (single-precision)"))
  (bind _output_get (set `self.ForwardSpeed` (+ 1.0 (`self.ForwardSpeed`))))
  (`self.K2_AddActorWorldOffset` (`KismetMathLibrary.MakeVector` (* DeltaSeconds (`self.ForwardSpeed`))) false true)
  (`KismetSystemLibrary.PrintString` (`KismetStringLibrary.Concat_StrStr` "speed:" (`KismetStringLibrary.Conv_DoubleToString` _output_get)) true true (struct :`R` 0.410272 :`G` 0.130708 :`B` 1.0 :`A` 1.0) 0.0))

(event `self.Sphere.OnComponentBeginOverlap`
  (params (OverlappedComponent :type "PrimitiveComponent Object Reference") (OtherActor :type "Actor Object Reference") (OtherComp :type "PrimitiveComponent Object Reference") (OtherBodyIndex :type Integer) (bFromSweep :type Boolean) (SweepResult :type "HitResult Structure (by ref)"))
  (bind _asbp_enemy (cast `/Game/InfiniteMatrix/Blueprints/BP_Enemy` OtherActor))
  (`self.K2_DestroyActor` _asbp_enemy)
  (`self.K2_DestroyActor`)
  (bind _asbp_player (cast `/Game/InfiniteMatrix/Blueprints/BP_Player` (`GameplayStatics.GetPlayerPawn` 0)))
  (`/Engine/EditorBlueprintResources/StandardMacros.DoOnce` false
    (:`Completed`
      (bind _output_get (set `/Game/InfiniteMatrix/Blueprints/BP_Player.Score` (+ (`/Game/InfiniteMatrix/Blueprints/BP_Player.Score` _asbp_player) 10) _asbp_player))
      (`KismetSystemLibrary.PrintString` (`KismetStringLibrary.Concat_StrStr` "Score :" (`KismetStringLibrary.Conv_IntToString` _output_get)) true true (struct :`R` 1.0 :`G` 0.895524 :`A` 1.0)))))

(fn `UserConstructionScript`)