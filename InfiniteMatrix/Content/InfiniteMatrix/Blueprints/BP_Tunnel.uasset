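; Tunnel segment for an endless obstacle run, with a rotating holed wall, a randomly placed health pack and a spawned BP_Enemy.
; Passing the trigger adds score, while hitting the wall costs health, shakes the camera and can show restart; both spawn the next tunnel and destroy this one.
; The pack heals with a brief UMG flash.
; RandomizeWall, not called here, varies hole mesh, roll and color through a dynamic material.
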(event `self.ReceiveBeginPlay`
  (`|ExecutionSequence`
    (:`then_0`
      (`self.RandomizeHealthPack`))
    (:`then_1`
      (`self.RandomizeEnemy`))))

(event `self.ReceiveTick`
  (params (DeltaSeconds :type "Float (single-precision)"))
  (`SceneComponent.K2_AddLocalRotation` (`self.WallMesh`) (`KismetMathLibrary.MakeRotator` (* DeltaSeconds (`self.RotateSpeed`))) false false))

(event `self.TriggerZone.OnComponentBeginOverlap`
  (params (OverlappedComponent :type "PrimitiveComponent Object Reference") (OtherActor :type "Actor Object Reference") (OtherComp :type "PrimitiveComponent Object Reference") (OtherBodyIndex :type Integer) (bFromSweep :type Boolean) (SweepResult :type "HitResult Structure (by ref)"))
  (bind _asbp_player (cast `/Game/InfiniteMatrix/Blueprints/BP_Player` OtherActor))
  (`/Engine/EditorBlueprintResources/StandardMacros.DoOnce` false
    (:`Completed`
      (set `/Game/InfiniteMatrix/Blueprints/BP_Player.Score` (+ (`/Game/InfiniteMatrix/Blueprints/BP_Player.Score` _asbp_player) 10) _asbp_player)
      (`/Game/InfiniteMatrix/Blueprints/BP_TunnelSpawner.SpawnTunnelAtSpawnPoint` (`self.TunnelSpawner`))
      (`self.K2_DestroyActor`)
      (bind _spawn_enemy (`self.Spawn_Enemy`)
        (:`then`
          (`self.K2_DestroyActor` _spawn_enemy))
        (:`else`)))))

(event `self.WallMesh.OnComponentHit`
  (params (HitComponent :type "PrimitiveComponent Object Reference") (OtherActor :type "Actor Object Reference") (OtherComp :type "PrimitiveComponent Object Reference") (NormalImpulse :type "Vector Structure") (Hit :type "HitResult Structure (by ref)"))
  (bind _asbp_player (cast `/Game/InfiniteMatrix/Blueprints/BP_Player` OtherActor))
  (set `/Game/InfiniteMatrix/Blueprints/BP_Player.Health` (`KismetMathLibrary.FClamp` (- (`/Game/InfiniteMatrix/Blueprints/BP_Player.Health` _asbp_player) 20.0) 0.0 100.0) _asbp_player)
  (`/Game/InfiniteMatrix/Blueprints/BP_TunnelSpawner.SpawnTunnelAtSpawnPoint` (`self.TunnelSpawner`))
  (`self.K2_DestroyActor`)
  (`|ExecutionSequence`
    (:`then_0`
      (if (== (`/Game/InfiniteMatrix/Blueprints/BP_Player.Health` _asbp_player) 0.0)
        (`/Game/InfiniteMatrix/Blueprints/BP_Player.DisplayRestart` _asbp_player)))
    (:`then_1`
      (bind _spawn_enemy (`self.Spawn_Enemy`)
        (:`then`
          (`self.K2_DestroyActor` _spawn_enemy))
        (:`else`)))
    (:`then_2`
      (`/Game/InfiniteMatrix/Blueprints/BP_Player.camerashake` _asbp_player 2.0))))

(event `self.HealthPack.OnComponentBeginOverlap`
  (params (OverlappedComponent :type "PrimitiveComponent Object Reference") (OtherActor :type "Actor Object Reference") (OtherComp :type "PrimitiveComponent Object Reference") (OtherBodyIndex :type Integer) (bFromSweep :type Boolean) (SweepResult :type "HitResult Structure (by ref)"))
  (bind _asbp_player (cast `/Game/InfiniteMatrix/Blueprints/BP_Player` OtherActor))
  (set `/Game/InfiniteMatrix/Blueprints/BP_Player.Health` (+ (`/Game/InfiniteMatrix/Blueprints/BP_Player.Health` _asbp_player) 10.0) _asbp_player)
  (`ActorComponent.K2_DestroyComponent` (`self.HealthPack`))
  (bind _returnvalue (`|CreateWidget` "/Game/InfiniteMatrix/UI/UMG_gettingH.UMG_gettingH_C" (`GameplayStatics.GetPlayerController` 0)))
  (`UserWidget.AddToViewport` _returnvalue 0)
  (`|ExecutionSequence`
    (:`then_0`
      (bind (_direction _time_track) (`Timeline|timeline`)
        (:`Update`
          (`/Game/InfiniteMatrix/UI/UMG_gettingH.Color` _returnvalue _time_track))))
    (:`then_1`
      (`KismetSystemLibrary.Delay` 0.6)
      (`Widget.RemoveFromParent` _returnvalue))))

(event `self.WallMesh.OnComponentBeginOverlap`
  (params (OverlappedComponent :type "PrimitiveComponent Object Reference") (OtherActor :type "Actor Object Reference") (OtherComp :type "PrimitiveComponent Object Reference") (OtherBodyIndex :type Integer) (bFromSweep :type Boolean) (SweepResult :type "HitResult Structure (by ref)"))
  (bind _asbp_shoot (cast `/Game/InfiniteMatrix/Blueprints/BP_Shoot` OtherActor))
  (`self.K2_DestroyActor` _asbp_shoot))

(event `self.HealthPack.OnComponentEndOverlap`
  (params (OverlappedComponent :type "PrimitiveComponent Object Reference") (OtherActor :type "Actor Object Reference") (OtherComp :type "PrimitiveComponent Object Reference") (OtherBodyIndex :type Integer))
  (bind _asbp_shoot (cast `/Game/InfiniteMatrix/Blueprints/BP_Shoot` OtherActor))
  (`self.K2_DestroyActor` _asbp_shoot))

(fn `RandomizeEnemy`
  (locals (NewLocalVar :type "Transform Structure"))
  (`SceneComponent.K2_AddLocalTransform` (`self.Enemy`) (`KismetMathLibrary.MakeTransform` (`KismetMathLibrary.MakeVector` (`KismetMathLibrary.RandomFloatInRange` 100.0 1200.0) (`KismetMathLibrary.RandomFloatInRange` -250.0 250.0) (`KismetMathLibrary.RandomFloatInRange` -200.0 200.0)) (`KismetMathLibrary.MakeRotator` 0.0 0.0 (`KismetMathLibrary.RandomFloatInRange` -90.0 90.0)) (5.0 5.0 5.0)) false false)
  (bind _returnvalue (`|SpawnActorFromClass` "/Game/InfiniteMatrix/Blueprints/BP_Enemy.BP_Enemy_C" (`KismetMathLibrary.MakeTransform` (`SceneComponent.K2_GetComponentLocation` (`self.Enemy`)) (struct :`Yaw` 90.0) (5.0 5.0 5.0)) "Undefined" "OverrideRootScale" null null))
  (set `self.Spawn_Enemy` _returnvalue))

(fn `RandomizeHealthPack`
  (`StaticMeshComponent.SetStaticMesh` (`self.HealthPack`) (select `bool` (`KismetMathLibrary.RandomBool`) :`false` "/Game/InfiniteMatrix/Meshes/Medkit.Medkit" :!type "StaticMesh Object Reference"))
  (`SceneComponent.K2_AddLocalTransform` (`self.HealthPack`) (`KismetMathLibrary.MakeTransform` (`KismetMathLibrary.MakeVector` (`KismetMathLibrary.RandomFloatInRange` 100.0 1200.0) (`KismetMathLibrary.RandomFloatInRange` -250.0 250.0) (`KismetMathLibrary.RandomFloatInRange` -200.0 200.0)) (struct) (0.5 0.5 0.5)) false false))

(fn `RandomizeWall`
  (bind _wallmesh (`self.WallMesh`))
  (`StaticMeshComponent.SetStaticMesh` _wallmesh (select `int` (`KismetMathLibrary.RandomIntegerInRange` 0 3) :`0` "/Game/InfiniteMatrix/Meshes/SM_Hole_01.SM_Hole_01" :`1` "/Game/InfiniteMatrix/Meshes/SM_Hole_02.SM_Hole_02" :`2` "/Game/InfiniteMatrix/Meshes/SM_Hole_03.SM_Hole_03" :`3` "/Game/InfiniteMatrix/Meshes/SM_Hole_04.SM_Hole_04" :!type "StaticMesh Object Reference"))
  (`SceneComponent.K2_AddLocalRotation` (`self.WallMesh`) (`KismetMathLibrary.MakeRotator` (`KismetMathLibrary.RandomFloatInRange` 0.0 360.0)) false false)
  (bind _returnvalue (`PrimitiveComponent.CreateDynamicMaterialInstance` _wallmesh 0 "/Game/InfiniteMatrix/Materials/MI_Hole.MI_Hole" "None"))
  (`MaterialInstanceDynamic.SetVectorParameterValue` _returnvalue "Color" (make `LinearColor` (`KismetMathLibrary.RandomFloat`) (`KismetMathLibrary.RandomFloat`) (`KismetMathLibrary.RandomFloat`) 1.0)))

(fn `UserConstructionScript`)